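; Game mode that sets up a match by registering the player and spawning AI opponents, then drives the circle timer.
; On BeginPlay it builds a grid of elevated spawn transforms, shuffles it and spawns AI at the first entries, avoiding overlapping picks.
; The player and AI are tracked in an alive-characters list, with AI also kept in their own list.
; A looping one-second timer calls the game state's circle update, leaving Tick empty.
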(event Custom|MainTimer
  (bind _asbp_project_one_game_state (Utilities|Casting|CastToBP_ProjectOneGameState (Game|GetGameState)))
  (Default|UpdateCircleMainTimer _asbp_project_one_game_state))

(event EventBeginPlay
  (bind _asproject_one_character (Utilities|Casting|CastToProjectOneCharacter (Pawn|GetControlledPawn (Game|GetPlayerController 0))))
  (bind _output_get (Variables|Default|Setplayer _asproject_one_character))
  (Utilities|Array|Add (Variables|Default|GetAliveChracters) _output_get)
  (Utilities|Time|SetTimerbyEvent (delegate Custom|MainTimer) 1.0 true)
  (for _index (range 0 9)
    (for _index_2 (range 0 9)
      (Utilities|Array|Add (Variables|Default|GetPlayerSpawnArrays) (Math|Transform|MakeTransform (Math|Vector|MakeVector (- (* _index (Variables|Default|GetGridDistance)) 4.6e+04) (- (* _index_2 (Variables|Default|GetGridDistance)) 4.6e+04) 5e+03)))))
  (Utilities|Array|Shuffle (Variables|Default|GetPlayerSpawnArrays))
  (for _index_3 (range 0 18)
    (bind _returnvalue (Game|SpawnActorfromClass "/Script/ProjectOne.AICharacter" (Utilities|Array|Get(acopy) (Variables|Default|GetPlayerSpawnArrays) _index_3) "Undefined" 0 0))
    (Utilities|Array|Add (Variables|Default|GetAIChracters) _returnvalue)
    (Utilities|Array|Add (Variables|Default|GetAliveChracters) _returnvalue))
  (Utilities|Array|Clear (Variables|Default|GetPlayerSpawnArrays)))

(event EventTick
  (params (DeltaSeconds :type Float%20%28single-precision%29)))

(fn ConstructionScript)