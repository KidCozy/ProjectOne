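; Player controller for ProjectOne that toggles a world map widget and exposes pawn placement data.
; The WoldMap input action drives a FlipFlop that adds or removes WidgetBP_WorldMap from the viewport, creating and caching it on first use.
; GetPawnPosition returns the controlled pawn's location and rotation with MapSize, falling back to a far-off position and zero rotation when no valid pawn exists.
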(event EventTick
  (params (DeltaSeconds :type Float%20%28single-precision%29)))

(event Input|ActionEvents|InputActionWoldMap
  (params (Key :type Key%20Structure))
  (bind _self self)
  (:Pressed
    (Utilities|FlowControl|FlipFlop
      (:A
        (Utilities|IsValid (Variables|Default|GetWidgetBP_WorldMap)
          (:Is%20Valid
            (UserInterface|Viewport|AddtoViewport (Variables|Default|GetWidgetBP_WorldMap) 0))
          (:Is%20Not%20Valid
            (bind _returnvalue (UserInterface|CreateWidget "/Game/ProjectOneBlueprint/WidgetBP_WorldMap.WidgetBP_WorldMap_C" _self _self))
            (bind _output_get (Variables|Default|SetWidgetBP_WorldMap _returnvalue))
            (UserInterface|Viewport|AddtoViewport _output_get 0))))
      (:B
        (Utilities|IsValid (Variables|Default|GetWidgetBP_WorldMap)
          (:Is%20Valid
            (Widget|RemovefromParent (Variables|Default|GetWidgetBP_WorldMap))))))))

(fn ConstructionScript)

(fn GetPawnPosition
  (bind _returnvalue (Pawn|GetControlledPawn))
  (bind _mapsize (Variables|Default|GetMapSize))
  (Utilities|IsValid _returnvalue
    (:Is%20Valid
      (return (Transformation|GetActorLocation _returnvalue) _mapsize (Transformation|GetActorRotation _returnvalue)))
    (:Is%20Not%20Valid
      (return "100000000376832.000000,1000.000000, 0" _mapsize "0, 0, 0"))))