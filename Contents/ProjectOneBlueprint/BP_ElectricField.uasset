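; BP_ElectricField is an actor that draws the current circle, apparently a battle-royale-style electric zone boundary, as a tall scaled static mesh.
; Each Tick it reads visibility, position and radius from BP_ProjectOneGameState and applies them to the mesh and actor transform.
; The radius becomes an XY scale (radius / 100 × 2) with a very large fixed Z scale, forming a column.
; It holds no zone or damage logic of its own.
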(event EventBeginPlay)

(event Collision|EventActorBeginOverlap
  (params (OtherActor :type Actor%20Object%20Reference)))

(event EventTick
  (params (DeltaSeconds :type Float%20%28single-precision%29))
  (bind _asbp_project_one_game_state (Utilities|Casting|CastToBP_ProjectOneGameState (Game|GetGameState)))
  (Rendering|SetVisibility (Variables|Default|GetStaticMesh) (Variables|/Game/ProjectOneBlueprint/BP_ProjectOneGameState.BP_ProjectOneGameState_C|GetVisibleCurrentCircle _asbp_project_one_game_state) true)
  (Transformation|SetActorLocation (Variables|/Game/ProjectOneBlueprint/BP_ProjectOneGameState.BP_ProjectOneGameState_C|GetCurrentCirclePosition _asbp_project_one_game_state) false false)
  (Transformation|SetActorScale3D (Math|Vector|MakeVector (* (/ (Variables|/Game/ProjectOneBlueprint/BP_ProjectOneGameState.BP_ProjectOneGameState_C|GetCurrentCircleRadius _asbp_project_one_game_state) 1e+02) 2.0) (* (/ (Variables|/Game/ProjectOneBlueprint/BP_ProjectOneGameState.BP_ProjectOneGameState_C|GetCurrentCircleRadius _asbp_project_one_game_state) 1e+02) 2.0) 1e+03)))

(fn ConstructionScript)