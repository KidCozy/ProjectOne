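; Game state Blueprint that runs the phases of a shrinking circle zone, with a current and a target circle.
; UpdateCircleMainTimer counts down waiting and show times, reveals each circle, then activates the magnetic shrink.
; Tick reduces the radius by a fixed step per frame until it reaches the target, then hides the target circle and resets both countdowns.
; BeginPlay precomputes per-second position and radius deltas, which these graphs never use.
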(event Custom|UpdateCircleMainTimer
  (bind _result (Math|Integer|DecrementInt (Variables|Default|GetWaitingTime))
    (:%20%20
      (if (not (>= _result 0))
        (if (Variables|Default|GetVisibleTargetCircle)
          _
          (else
            (Variables|Default|SetVisibleTargetCircle true)))
        (bind _result_2 (Math|Integer|DecrementInt (Variables|Default|GetShowTime))
          (:%20%20
            (if (not (>= _result_2 0))
              (if (Variables|Default|GetVisibleCurrentCircle)
                (Variables|Default|SetbMagneticActivasion true)
                (else
                  (Variables|Default|SetVisibleCurrentCircle true))))))))))

(event EventBeginPlay
  (Variables|Default|SetDeltaPositionperSec (/ (- (Variables|Default|GetCurrentCirclePosition) (Variables|Default|GetTargetCirclePosition)) (Variables|Default|GetShrinkTime)))
  (Variables|Default|SetDeltaRadiusPerSec (/ (- (Variables|Default|GetTargetCircleRadius) (Variables|Default|GetCurrentCircleRadius)) (Math|Conversions|ToFloat(Integer) (Variables|Default|GetShrinkTime)))))

(event EventTick
  (params (DeltaSeconds :type Float%20%28single-precision%29))
  (if (Variables|Default|GetbMagneticActivasion)
    (Variables|Default|SetCurrentCircleRadius (- (Variables|Default|GetCurrentCircleRadius) 1e+01))
    (if (>= (Variables|Default|GetTargetCircleRadius) (Variables|Default|GetCurrentCircleRadius))
      (Variables|Default|SetbMagneticActivasion false)
      (if (Variables|Default|GetVisibleTargetCircle)
        (Variables|Default|SetVisibleTargetCircle false)
        (Variables|Default|SetWaitingTime 10)
        (Variables|Default|SetShowTime 10)))))

(fn ConstructionScript)